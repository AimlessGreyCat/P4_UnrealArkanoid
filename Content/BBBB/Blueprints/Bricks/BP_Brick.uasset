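; BP_Brick is a breakable brick that loses HP each time the ball hits it.
; When destroyed, it tells BP_GameModeBase to decrement the brick count and add its score value, with a random chance to spawn a BP_PowerUp at its location.
; A WBP_BrickHitPoints widget component shows remaining HP, updated on surviving hits and hidden at start for bricks without more than one HP.
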(event `/Game/BBBB/Blueprints/BP_BallHitReactionInterface.HitByBall`
  (bind _result (`/Engine/EditorBlueprintResources/StandardMacros.DecrementInt` (`self.HP`))
    (:`  `
      (if (<= _result 0)
        (`self.K2_DestroyActor`)
        (bind _asbp_game_mode_base (cast `/Game/BBBB/Blueprints/BP_GameModeBase` (`GameplayStatics.GetGameMode`)))
        (`/Game/BBBB/Blueprints/BP_GameModeBase.DecrementBrick` _asbp_game_mode_base)
        (`/Game/BBBB/Blueprints/BP_GameModeBase.UpdateScore` _asbp_game_mode_base (`self.ScoreValue`))
        (if (== (`KismetMathLibrary.RandomInteger` 10) 1)
          (`|SpawnActorFromClass` "/Game/BBBB/Blueprints/BP_PowerUp.BP_PowerUp_C" (`KismetMathLibrary.MakeTransform` (`self.K2_GetActorLocation`)) "Undefined" "OverrideRootScale" null null))
        (else
          (bind _aswbp_brick_hit_points (cast `/Game/BBBB/Widgets/WBP_BrickHitPoints` (`WidgetComponent.GetUserWidgetObject` (`self.HPText`))))
          (`/Game/BBBB/Widgets/WBP_BrickHitPoints.Update HP Text` _aswbp_brick_hit_points (`self.HP`)))))))

(event `self.ReceiveBeginPlay`
  (bind _aswbp_brick_hit_points (cast `/Game/BBBB/Widgets/WBP_BrickHitPoints` (`WidgetComponent.GetUserWidgetObject` (`self.HPText`))))
  (`/Game/BBBB/Widgets/WBP_BrickHitPoints.Update HP Text` _aswbp_brick_hit_points (`self.HP`))
  (if (not (> (`self.HP`) 1))
    (`SceneComponent.SetVisibility` (`self.HPText`) false false)))

(fn `UserConstructionScript`)