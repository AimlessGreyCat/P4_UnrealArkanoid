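; BP_PowerUp is a power-up capsule actor that picks one of three types at random on BeginPlay: Laser, Enlarge or Player.
; The chosen type sets the capsule's material and a single-letter text label so the kind is visible.
; It destroys itself on overlapping BP_LoseTrigger; this Blueprint contains no movement, pickup or effect logic.
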(event `self.ReceiveBeginPlay`
  (bind _output_get (set `self.PowerUpType` (select `int` (`KismetMathLibrary.RandomInteger` 3) :`0` "NewEnumerator0" :`1` "NewEnumerator1" :`2` "NewEnumerator2" :!type "/Game/BBBB/Enums/EPowerUps Enum")))
  (switch `/Game/BBBB/Enums/EPowerUps` _output_get
    (:`NewEnumerator0`
      (`PrimitiveComponent.SetMaterial` (`self.Capsule`) 0 "/Game/BBBB/Materials/MI_FlatColourRed.MI_FlatColourRed")
      (`TextRenderComponent.K2_SetText` (`self.PowerUpLetter`) "L"))
    (:`NewEnumerator1`
      (`PrimitiveComponent.SetMaterial` (`self.Capsule`) 0 "/Game/BBBB/Materials/MI_FlatColourBlue.MI_FlatColourBlue")
      (`TextRenderComponent.K2_SetText` (`self.PowerUpLetter`) "E"))
    (:`NewEnumerator2`
      (`PrimitiveComponent.SetMaterial` (`self.Capsule`) 0 "/Game/StarterContent/Materials/M_Metal_Chrome.M_Metal_Chrome")
      (`TextRenderComponent.K2_SetText` (`self.PowerUpLetter`) "P"))))

(event `self.ReceiveActorBeginOverlap`
  (params (OtherActor :type "Actor Object Reference"))
  (cast `/Game/BBBB/Blueprints/BP_LoseTrigger` OtherActor)
  (`self.K2_DestroyActor`))

(fn `UserConstructionScript`)