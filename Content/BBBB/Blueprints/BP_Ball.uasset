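; Breakout-style ball actor that moves along a direction while the GameMode is in a specific game state.
; Swept movement reflects off impact normals, while paddle hits set direction by the ball's offset from the paddle, yaw-clamped to ±70°.
; Other hit actors implementing the hit-reaction interface are notified.
; Overlapping a lose trigger decrements GameMode lives and, if any remain, resets the ball to spawn and hides it.
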(event `self.ReceiveBeginPlay`
  (`KismetMathLibrary.Vector_Normalize` (`self.Direction`))
  (set `self.SpawnPos` (`self.K2_GetActorLocation`))
  (bind _asbp_game_mode_base (cast `/Game/BBBB/Blueprints/BP_GameModeBase` (`GameplayStatics.GetGameMode`)))
  (set `self.GameModeRef` _asbp_game_mode_base))

(event `self.ReceiveTick`
  (params (DeltaSeconds :type "Float (single-precision)"))
  (if (`|EnumEquality` (`/Game/BBBB/Blueprints/BP_GameModeBase.CurrentGameState` (`self.GameModeRef`)) "NewEnumerator1")
    (bind _sweephitresult (`self.K2_AddActorWorldOffset` (* DeltaSeconds (* (`self.Direction`) (`self.Speed`))) true))
    (bind _asbp_paddle (cast `/Game/BBBB/Blueprints/BP_Paddle` (`.HitActor` (`GameplayStatics.BreakHitResult` _sweephitresult)))
      (:`then`
        (bind (_returnvalue_roll _returnvalue_pitch _returnvalue_yaw) (`KismetMathLibrary.BreakRotator` (`KismetMathLibrary.FindLookAtRotation` (`self.K2_GetActorLocation` _asbp_paddle) (`self.K2_GetActorLocation`))))
        (set `self.Direction` (`KismetMathLibrary.GetForwardVector` (`KismetMathLibrary.MakeRotator` 0.0 0.0 (`KismetMathLibrary.ClampAngle` _returnvalue_yaw -70.0 70.0)))))
      (:`CastFailed`
        (set `self.Direction` (`KismetMathLibrary.GetReflectionVector` (`self.Direction`) (`.ImpactNormal` (`GameplayStatics.BreakHitResult` _sweephitresult))))
        (if (`KismetSystemLibrary.DoesImplementInterface` (`.HitActor` (`GameplayStatics.BreakHitResult` _sweephitresult)) "/Game/BBBB/Blueprints/BP_BallHitReactionInterface.BP_BallHitReactionInterface_C")
          (message `/Game/BBBB/Blueprints/BP_BallHitReactionInterface.HitByBall` (`.HitActor` (`GameplayStatics.BreakHitResult` _sweephitresult))))))
    (else
      (`SceneComponent.SetVisibility` (`self.Ball`) (not (`|EnumEquality` (`/Game/BBBB/Blueprints/BP_GameModeBase.CurrentGameState` (`self.GameModeRef`)) "NewEnumerator4")) false))))

(event `self.ReceiveActorBeginOverlap`
  (params (OtherActor :type "Actor Object Reference"))
  (cast `/Game/BBBB/Blueprints/BP_LoseTrigger` OtherActor)
  (bind _asbp_game_mode_base (cast `/Game/BBBB/Blueprints/BP_GameModeBase` (`GameplayStatics.GetGameMode`)))
  (`/Game/BBBB/Blueprints/BP_GameModeBase.DecrementLives` _asbp_game_mode_base)
  (if (> (`/Game/BBBB/Blueprints/BP_GameModeBase.Lives` _asbp_game_mode_base) 0)
    (`self.K2_SetActorLocation` (`self.SpawnPos`))
    (set `self.Direction` (1.0 0.0 0.0))
    (`SceneComponent.SetVisibility` (`self.Ball`) false false)))

(fn `UserConstructionScript`)