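; Game mode for an Arkanoid-style brick breaker that owns lives, remaining bricks and the game state, and drives the HUD.
; On start it creates the HUD, counts placed bricks, caches the game instance holding the score, and runs a timed countdown.
; Losing a life either recenters the paddle or ends the game, while clearing all bricks shows victory and loads Level1 after a delay.
; Lives gained are capped, and score updates go to the game instance.
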(event `self.ReceiveBeginPlay`
  (bind _returnvalue (`|CreateWidget` "/Game/BBBB/Widgets/WBP_HUD.WBP_HUD_C"))
  (bind _output_get (set `self.HUDRef` _returnvalue))
  (`UserWidget.AddToViewport` _output_get 0)
  (bind _outactors (`GameplayStatics.GetAllActorsOfClass` "/Game/BBBB/Blueprints/Bricks/BP_Brick.BP_Brick_C"))
  (for _ _outactors
    (`/Engine/EditorBlueprintResources/StandardMacros.IncrementInt` (`self.BricksRemaining`)))
  (bind _asbp_arkanoid_game_instance (cast `/Game/BBBB/Blueprints/BP_ArkanoidGameInstance` (`GameplayStatics.GetGameInstance`)))
  (set `self.GameInstanceRef` _asbp_arkanoid_game_instance)
  (`self.Countdown`))

(event `Countdown`
  (set `self.CurrentGameState` "NewEnumerator0")
  (`/Game/BBBB/Widgets/WBP_HUD.UpdateAnnouncementText` (`self.HUDRef`))
  (`KismetSystemLibrary.Delay` 4.0)
  (set `self.CurrentGameState` "NewEnumerator1"))

(event `Respawn`
  (set `self.CurrentGameState` "NewEnumerator4")
  (`/Game/BBBB/Widgets/WBP_HUD.UpdateAnnouncementText` (`self.HUDRef`))
  (bind _asbp_paddle (cast `/Game/BBBB/Blueprints/BP_Paddle` (`GameplayStatics.GetPlayerPawn` 0)))
  (`/Game/BBBB/Blueprints/BP_Paddle.MoveToOrigin` _asbp_paddle))

(event `GameOver`
  (set `self.CurrentGameState` "NewEnumerator2")
  (`/Game/BBBB/Widgets/WBP_HUD.UpdateAnnouncementText` (`self.HUDRef`)))

(event `Victory`
  (set `self.CurrentGameState` "NewEnumerator3")
  (`/Game/BBBB/Widgets/WBP_HUD.UpdateAnnouncementText` (`self.HUDRef`))
  (`KismetSystemLibrary.Delay` 3.0)
  (`GameplayStatics.OpenLevel` "Level1"))

(event `Increment Lives`
  (bind _result (`/Engine/EditorBlueprintResources/StandardMacros.IncrementInt` (`self.Lives`))
    (:`  `
      (if (> _result 6)
        (bind _output_get (set `self.Lives` 6)))
      (`/Game/BBBB/Widgets/WBP_HUD.UpdateLives` (`self.HUDRef`) _output_get))))

(fn `DecrementBrick`
  (`/Engine/EditorBlueprintResources/StandardMacros.DecrementInt` (`self.BricksRemaining`)
    (:`  `
      (if (<= (`self.BricksRemaining`) 0)
        (`self.Victory`)))))

(fn `DecrementLives`
  (bind _result (`/Engine/EditorBlueprintResources/StandardMacros.DecrementInt` (`self.Lives`))
    (:`  `
      (`/Game/BBBB/Widgets/WBP_HUD.UpdateLives` (`self.HUDRef`) _result)
      (if (> (`self.Lives`) 0)
        (`self.Respawn`)
        (else
          (`self.GameOver`))))))

(fn `UpdateScore`
  (params (Value :type Integer))
  (set `/Game/BBBB/Blueprints/BP_ArkanoidGameInstance.Score` (+ (`/Game/BBBB/Blueprints/BP_ArkanoidGameInstance.Score` (`self.GameInstanceRef`)) Value) (`self.GameInstanceRef`))
  (`/Game/BBBB/Widgets/WBP_HUD.UpdateScoreText` (`self.HUDRef`)))

(fn `UserConstructionScript`)